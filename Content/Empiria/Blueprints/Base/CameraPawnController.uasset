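; Player controller for Empiria's camera navigation and building placement.
; On BeginPlay it spawns a construction manager and ghost building, then creates the main HUD.
; It drives the camera pawn with zoom-scaled axis movement, screen-edge scrolling, spring-arm zoom and gated mouse rotation.
; In building mode the ghost follows the cursor and rotates, and left click queues valid placements with the manager, while a temporary key spawns humans.
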(event `self.ReceiveBeginPlay`
  (bind _returnvalue (`KismetMathLibrary.MakeTransform` (0.0 0.0 0.0)))
  ;[1 1 1] Setup
  (`|ExecutionSequence`
    (:`then_0`
      (`self.ReferenceCasts`))
    (:`then_1`
      (bind _returnvalue_2 (`|SpawnActorFromClass` "/Game/Empiria/Blueprints/Construction/ConstructionManagerBP.ConstructionManagerBP_C" _returnvalue "AlwaysSpawn" "OverrideRootScale"))
      (set `self.ConstructionManagerReference` _returnvalue_2))
    (:`then_2`
      (bind _returnvalue_3 (`|SpawnActorFromClass` "/Game/Empiria/Blueprints/Buildings/GhostBuildingBP.GhostBuildingBP_C" _returnvalue "AlwaysSpawn" "OverrideRootScale" null self))
      (set `self.GhostBuildingReference` _returnvalue_3))
    (:`then_3`
      (`WidgetBlueprintLibrary.SetInputMode_GameAndUIEx` self null "LockOnCapture" false)
      (`self.CreateHUD`)
      (`UserWidget.AddToViewport` (`self.MainUI`) 0))))

(event `InputAxis|MoveForward`
  (params (AxisValue :type "Float (single-precision)"))
  ;[1 1 1] Camera movement
  ;;[1 1 1] Movement X
  (if (not (`self.DisableCamNav`))
    (`self.K2_SetActorTransform` (`self.CameraPawnReference`) (`KismetMathLibrary.MakeTransform` (`KismetMathLibrary.MakeVector` (.x (.location (`self.MovementX` AxisValue (`self.MoevementSpeedCalculation`) (`self.FastMoveMultiplier`) (`self.CameraPawnReference`)))) (.y (.location (`self.MovementX` AxisValue (`self.MoevementSpeedCalculation`) (`self.FastMoveMultiplier`) (`self.CameraPawnReference`)))) 150.0) (.rotation (`self.MovementX` AxisValue (`self.MoevementSpeedCalculation`) (`self.FastMoveMultiplier`) (`self.CameraPawnReference`))) (.scale (`self.MovementX` AxisValue (`self.MoevementSpeedCalculation`) (`self.FastMoveMultiplier`) (`self.CameraPawnReference`)))) true false)))

(event `InputAction|ZoomIn`
  (params (Key :type "Key Structure" :default "AnyKey"))
  (bind _springarm (`/Game/Empiria/Blueprints/Base/CameraPawn.SpringArm` (`self.CameraPawnReference`)))
  ;[1 1 1] Camera movement
  ;;[1 1 1] Zooming
  (:`Pressed`
    (set `SpringArmComponent.TargetArmLength` (`KismetMathLibrary.FClamp` (- (`SpringArmComponent.TargetArmLength` _springarm) (`self.ZommSensitivity`)) 200.0 (`self.MaxZoomDistance`)) _springarm)))

(event `InputAxisKey|MouseX`
  (params (AxisValue :type "Float (single-precision)"))
  ;[1 1 1] Camera movement
  ;;[1 1 1] Pan X
  (`/Engine/EditorBlueprintResources/StandardMacros.Gate` true :!label _label
    (:`Exit`
      (`self.K2_SetActorRotation` (`self.CameraPawnReference`) (`KismetMathLibrary.MakeRotator` (.roll (`self.K2_GetActorRotation` (`self.CameraPawnReference`))) (.pitch (`self.K2_GetActorRotation` (`self.CameraPawnReference`))) (+ (.yaw (`self.K2_GetActorRotation` (`self.CameraPawnReference`))) (* (`self.PanSensitivity`) AxisValue))) false))))

(event `InputAction|Pan`
  (params (Key :type "Key Structure" :default "AnyKey"))
  ;[1 1 1] Camera movement
  ;;[1 1 1] Pan X
  (:`Pressed`
    (set `self.DisableCamNav` false)
    (goto _label :!via `Open`))
  (:`Released`
    (set `self.DisableCamNav` false)
    (goto _label :!via `Close`)))

(event `InputAction|ZoomOut`
  (params (Key :type "Key Structure" :default "AnyKey"))
  (bind _springarm (`/Game/Empiria/Blueprints/Base/CameraPawn.SpringArm` (`self.CameraPawnReference`)))
  ;[1 1 1] Camera movement
  ;;[1 1 1] Zooming
  (:`Pressed`
    (set `SpringArmComponent.TargetArmLength` (`KismetMathLibrary.FClamp` (+ (`SpringArmComponent.TargetArmLength` _springarm) (`self.ZommSensitivity`)) 200.0 (`self.MaxZoomDistance`)) _springarm)))

(event `InputAxis|MoveRight`
  (params (AxisValue :type "Float (single-precision)"))
  ;[1 1 1] Camera movement
  ;;[1 1 1] MovementY
  (if (not (`self.DisableCamNav`))
    (`self.K2_SetActorTransform` (`self.CameraPawnReference`) (`KismetMathLibrary.MakeTransform` (`KismetMathLibrary.MakeVector` (.x (.location (`self.MovementY` AxisValue (`self.MoevementSpeedCalculation`) (`self.FastMoveMultiplier`) (`self.CameraPawnReference`)))) (.y (.location (`self.MovementY` AxisValue (`self.MoevementSpeedCalculation`) (`self.FastMoveMultiplier`) (`self.CameraPawnReference`)))) 150.0) (.rotation (`self.MovementY` AxisValue (`self.MoevementSpeedCalculation`) (`self.FastMoveMultiplier`) (`self.CameraPawnReference`))) (.scale (`self.MovementY` AxisValue (`self.MoevementSpeedCalculation`) (`self.FastMoveMultiplier`) (`self.CameraPawnReference`)))) false false)))

(event `InputAxisKey|MouseY`
  (params (AxisValue :type "Float (single-precision)"))
  ;[1 1 1] Camera movement
  ;;[1 1 1] Pan Y
  (`/Engine/EditorBlueprintResources/StandardMacros.Gate` true :!label _label_2
    (:`Exit`
      (`self.K2_SetActorRotation` (`self.CameraPawnReference`) (`KismetMathLibrary.MakeRotator` (.roll (`self.K2_GetActorRotation` (`self.CameraPawnReference`))) (`KismetMathLibrary.FClamp` (+ (.pitch (`self.K2_GetActorRotation` (`self.CameraPawnReference`))) (* (`self.PanSensitivity`) AxisValue)) 0.0 70.0) (.yaw (`self.K2_GetActorRotation` (`self.CameraPawnReference`)))) false))))

(event `InputAxisKey|MouseX`
  (params (AxisValue :type "Float (single-precision)"))
  ;[1 1 1] Camera movement
  ;;[1 1 1] Screen edge movement
  (bind (_deltaxspeed _deltayspeed) (`self.ScreenEdgeMovement` :!label _label_3))
  (`self.K2_AddActorLocalOffset` (`self.CameraPawnReference`) (`KismetMathLibrary.MakeVector` _deltayspeed _deltaxspeed) true false))

(event `InputAction|Pan`
  (params (Key :type "Key Structure" :default "AnyKey"))
  ;[1 1 1] Camera movement
  ;;[1 1 1] Pan Y
  (:`Pressed`
    (set `self.DisableCamNav` false)
    (goto _label_2 :!via `Open`))
  (:`Released`
    (set `self.DisableCamNav` false)
    (goto _label_2 :!via `Close`)))

(event `InputAxisKey|MouseY`
  (params (AxisValue :type "Float (single-precision)"))
  ;[1 1 1] Camera movement
  ;;[1 1 1] Screen edge movement
  (goto _label_3 :!via `MouseY`))

(event `InputAction|PanReset`
  (params (Key :type "Key Structure" :default "AnyKey"))
  ;[1 1 1] Camera movement
  ;;[1 1 1] Reset Pan
  (:`Pressed`
    (`self.K2_SetActorRotation` (`self.CameraPawnReference`) (`KismetMathLibrary.MakeRotator` (.roll (`self.K2_GetActorRotation` (`self.CameraPawnReference`))) 0.0 (.yaw (`self.K2_GetActorRotation` (`self.CameraPawnReference`)))) false)))

(event `Key|LeftShift`
  (params (Key :type "Key Structure" :default "AnyKey"))
  ;[1 1 1] Camera movement
  ;;[1 1 1] Speed up
  (:`Pressed`
    (set `self.FastMoveMultiplier` 6.0))
  (:`Released`
    (set `self.FastMoveMultiplier` 1.0)))

(event `InputAction|Deselect`
  (params (Key :type "Key Structure" :default "AnyKey"))
  ;[1 1 1] Deselect
  (:`Pressed`
    (if (`self.BuildingModeActive`)
      (`/Game/Empiria/Blueprints/Buildings/GhostBuildingBP.KillGhost` (`self.GhostBuildingReference`))
      (set `self.BuildingModeActive` false))))

(event `Key|LeftMouseButton`
  (params (Key :type "Key Structure" :default "AnyKey"))
  ;[1 1 1] Create building (LMB)
  (:`Pressed`
    (if (and (`self.BuildingModeActive`) (`/Game/Empiria/Blueprints/Buildings/GhostBuildingBP.CanBeBuilt` (`self.GhostBuildingReference`)))
      (bind _constructionstruct (`/Game/Empiria/Blueprints/Buildings/GhostBuildingBP.GetConstructionStruct` (`self.GhostBuildingReference`)))
      (`/Game/Empiria/Blueprints/Construction/ConstructionManagerBP.QueueConstruction` (`self.ConstructionManagerReference`) _constructionstruct)
      (`/Game/Empiria/Blueprints/Buildings/GhostBuildingBP.KillGhost` (`self.GhostBuildingReference`)))))

(event `self.ReceiveTick`
  (params (DeltaSeconds :type "Float (single-precision)"))
  ;[1 1 1] Set GhostBuilding World Cursor Location
  (`|ExecutionSequence`
    (:`then_0`
      (if (`self.BuildingModeActive`)
        (if (!= (`self.GhostBuildingReference`) null)
          (set `/Game/Empiria/Blueprints/Buildings/GhostBuildingBP.CursorWorldLocation` (`/Game/Empiria/Libs/Functions.GetCursorWorldPosition` self (`self.GetSightDistance`)) (`self.GhostBuildingReference`)))))))

(event `InputAction|Rotate`
  (params (Key :type "Key Structure" :default "AnyKey"))
  (bind _ghostbuildingreference (`self.GhostBuildingReference`))
  ;[1 1 1] Handle building Rotation
  (:`Pressed`
    (if (`self.BuildingModeActive`)
      (`/Game/Empiria/Blueprints/Buildings/GhostBuildingBP.StartBuildingRotation` _ghostbuildingreference false)))
  (:`Released`
    (`/Game/Empiria/Blueprints/Buildings/GhostBuildingBP.EndBuildingRotation` _ghostbuildingreference :!label _label_4)))

(event `Key|V`
  (params (Key :type "Key Structure" :default "AnyKey"))
  (bind (_location_x _location_y) (`KismetMathLibrary.BreakVector` (`/Game/Empiria/Libs/Functions.GetCursorWorldPosition` self 5000.0)))
  ;[1 1 1] [TMP] place human
  (:`Pressed`
    (`|SpawnActorFromClass` "/Game/Empiria/Blueprints/AI/HumanBP.HumanBP_C" (`KismetMathLibrary.MakeTransform` (`KismetMathLibrary.MakeVector` _location_x _location_y 93.0)) "Undefined" "OverrideRootScale")))

(event `InputAction|RotateCCW`
  (params (Key :type "Key Structure" :default "AnyKey"))
  ;[1 1 1] Handle building Rotation
  (:`Pressed`
    (if (`self.BuildingModeActive`)
      (`/Game/Empiria/Blueprints/Buildings/GhostBuildingBP.StartBuildingRotation` (`self.GhostBuildingReference`) true)))
  (:`Released`
    (goto _label_4)))

(fn `GetSightDistance`
  (returns (Distance :type "Float (double-precision)"))
  (locals (DefaultSightDistance :type "Float (double-precision)" :default 2000.0))
  (return (+ (`SpringArmComponent.TargetArmLength` (`/Game/Empiria/Blueprints/Base/CameraPawn.SpringArm` (`self.CameraPawnReference`))) (`local.DefaultSightDistance`))))

(fn `MoevementSpeedCalculation`
  (returns (MoveSensitivity :type "Float (double-precision)"))
  (return (`KismetMathLibrary.FClamp` (/ (`SpringArmComponent.TargetArmLength` (`/Game/Empiria/Blueprints/Base/CameraPawn.SpringArm` (`self.CameraPawnReference`))) 10.0) 10.0 100.0)))

(fn `SetCalendar`
  (params (GameDate :type "Array of Integer (by ref)"))
  (returns (Success :type Boolean))
  (return false))

(fn `SetClock`
  (params (GameTime :type "Array of Integer (by ref)"))
  (returns (Success :type Boolean))
  (return false))

(fn `SetGameSpeed`
  (params (GameSpeed :type Integer))
  (returns (Success :type Boolean))
  (return false))

(fn `UserConstructionScript`)