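; Game state for Empiria that keeps the in-game clock and its selectable speed.
; Each tick advances CurrentGameTime by real delta seconds scaled by the current speed's Timespan in the GameSpeeds map, which acts as game time per real second.
; Speed changes by enum steps or directly by key, applied only when the map contains that key.
; BeginPlay also caches the player's CameraPawnController.
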(event `self.ReceiveBeginPlay`
  ;[1 1 1] Init
  (`|ExecutionSequence`
    (:`then_0`
      (`self.SetReferences`))))

(event `self.ReceiveTick`
  (params (DeltaSeconds :type "Float (single-precision)"))
  (`self.UpdateGameTime` DeltaSeconds))

(fn `GetDeltaGameTime`
  (params (Deltaseconds :type "Float (double-precision)"))
  (returns (ReturnValue :type "Timespan Structure"))
  (return (`KismetMathLibrary.MakeTimespan` 0 0 0 0 (`KismetMathLibrary.FTrunc` (* Deltaseconds (`KismetMathLibrary.GetTotalMilliseconds` (`BlueprintMapLibrary.Map_Find` (`self.GameSpeeds`) (`self.CurrentGameSpeed`))))))))

(fn `IncrementGameSpeedBy`
  (params (Steps :type Integer))
  (locals (NewCandidate :type Integer))
  (bind _output_get (set `local.NewCandidate` (+ (`KismetMathLibrary.Conv_ByteToInt` (`self.CurrentGameSpeed`)) Steps)))
  (if (and (>= _output_get 0) (<= _output_get (enumcount `/Game/Empiria/Enums/GameSpeedsEnum`)))
    (`self.SetGameSpeedTo` (cast `/Game/Empiria/Enums/GameSpeedsEnum` (`KismetMathLibrary.Conv_IntToByte` (`local.NewCandidate`))))))

(fn `SetGameSpeedTo`
  (params (Key :type "/Game/Empiria/Enums/GameSpeedsEnum Enum (by ref)"))
  (if (`.ReturnValue` (`BlueprintMapLibrary.Map_Find` (`self.GameSpeeds`) Key))
    (set `self.CurrentGameSpeed` Key)))

(fn `UpdateGameTime`
  (params (DeltaSeconds :type "Float (double-precision)"))
  (bind _returnvalue (`self.GetDeltaGameTime` DeltaSeconds))
  (set `self.CurrentGameTime` (+ (`self.CurrentGameTime`) _returnvalue)))

(fn `UserConstructionScript`)