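; Behavior tree task for human AI, named for assigning construction work, that so far only checks whether any construction proxies exist.
; On execute it runs a ReferenceCast helper for the AIHumanController and HumanBP references, casting only when they are not valid.
; It reads the proxy list through the controller's camera controller and construction manager, finishing successfully when empty.
; When proxies exist, no assignment logic runs and the task never finishes.
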(event `self.ReceiveExecuteAI`
  (params (OwnerController :type "AIController Object Reference") (ControlledPawn :type "Pawn Object Reference"))
  (`/Engine/EditorBlueprintResources/StandardMacros.IsValid` (`self.Controller`)
    (:`Is Valid`
      _)
    (:`Is Not Valid`
      (bind _asaihuman_controller (cast `/Game/Empiria/Blueprints/AI/AIHumanController` OwnerController))
      (set `self.Controller` _asaihuman_controller)))
  (`/Engine/EditorBlueprintResources/StandardMacros.IsValid` (`self.Pawn`)
    (:`Is Valid`
      _)
    (:`Is Not Valid`
      (bind _ashuman_bp (cast `/Game/Empiria/Blueprints/AI/HumanBP` ControlledPawn))
      (set `self.Pawn` _ashuman_bp)))
  (if (not (> (`KismetArrayLibrary.Array_Length` (`/Game/Empiria/Blueprints/Construction/ConstructionManagerBP.Proxies` (`/Game/Empiria/Blueprints/Base/CameraPawnController.ConstructionManagerReference` (`/Game/Empiria/Blueprints/AI/AIHumanController.CameraControllerRef` (`self.Controller`))))) 0))
    (`self.FinishExecute` true)))

(fn `AIHumanExecutionReferenceCast`
  (params (Controller :type "Object Object Reference") (Pawn :type "Object Object Reference"))
  (returns (AIController :type "/Game/Empiria/Blueprints/AI/AIHumanController Object Reference") (HumanPawn :type "/Game/Empiria/Blueprints/AI/HumanBP Object Reference"))
  (`/Engine/EditorBlueprintResources/StandardMacros.IsValid` (`self.Controller`)
    (:`Is Valid`
      _)
    (:`Is Not Valid`
      (bind _asaihuman_controller (cast `/Game/Empiria/Blueprints/AI/AIHumanController` Controller))
      (bind _output_get (set `self.Controller` _asaihuman_controller))))
  (`/Engine/EditorBlueprintResources/StandardMacros.IsValid` (`self.Pawn`)
    (:`Is Valid`
      _)
    (:`Is Not Valid`
      (bind _ashuman_bp (cast `/Game/Empiria/Blueprints/AI/HumanBP` Pawn))
      (bind _output_get_2 (set `self.Pawn` _ashuman_bp))))
  (return _output_get _output_get_2))