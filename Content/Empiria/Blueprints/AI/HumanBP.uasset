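; HumanBP is an AI-folder human that receives a random sex and matching name, with its event graph left empty.
; The construction script rolls the sex, tints a dynamic UE4 mannequin body material male or female, and fills InfoStruct, so values re-roll whenever construction reruns.
; Names come from random entries in separate male and female name enums, converted to strings.
; GetGender and GetName expose the stored results.
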(fn `GetGender`
  (returns (Gender :type "/Game/Empiria/Enums/SexesEnum Enum"))
  (bind _infostruct_sex (break `/Game/Empiria/Structs/HumanPawnInfo` (`self.InfoStruct`)))
  (return _infostruct_sex))

(fn `GetName`
  (returns (Name :type String))
  (bind (_infostruct_sex _infostruct_name) (break `/Game/Empiria/Structs/HumanPawnInfo` (`self.InfoStruct`)))
  (return _infostruct_name))

(fn `InitRandomName`
  (params (Sex :type "/Game/Empiria/Enums/SexesEnum Enum"))
  (returns (RandomName :type String))
  (if (`|EnumEquality` Sex "NewEnumerator0")
    (return (`|GetEnumeratorNameAsString` (cast `/Game/Empiria/Enums/PeopleNamesMaleEnum` (`KismetMathLibrary.Conv_IntToByte` (`KismetMathLibrary.RandomIntegerInRange` 0 (- (enumcount `/Game/Empiria/Enums/PeopleNamesMaleEnum`) 1))))))
    (else
      (return (`|GetEnumeratorNameAsString` (cast `/Game/Empiria/Enums/PeopleNamesFemaleEnum` (`KismetMathLibrary.Conv_IntToByte` (`KismetMathLibrary.RandomIntegerInRange` 0 (- (enumcount `/Game/Empiria/Enums/PeopleNamesFemaleEnum`) 1)))))))))

(fn `RandomCharacterFeatures`
  (locals (MaterialInstance :type "MaterialInstanceDynamic Object Reference") (RandomSex :type "/Game/Empiria/Enums/SexesEnum Enum") (FemaleColor :type "LinearColor Structure" :default (struct :`R` 0.155 :`G` 0.009937 :`B` 0.0031)) (MaleColor :type "LinearColor Structure" :default (struct :`R` 0.033934 :`G` 0.039201 :`B` 0.055)))
  (bind _materialinstance (`local.MaterialInstance`))
  (bind _returnvalue (`PrimitiveComponent.CreateDynamicMaterialInstance` (`self.Mesh`) 0 "/Game/Empiria/Models/Mannequin/Character/Materials/M_UE4Man_Body_Inst.M_UE4Man_Body_Inst"))
  (set `local.MaterialInstance` _returnvalue)
  (bind _output_get (set `local.RandomSex` (cast `/Game/Empiria/Enums/SexesEnum` (`KismetMathLibrary.Conv_IntToByte` (`KismetMathLibrary.RandomIntegerInRange` 0 1)))))
  (if (`|EnumEquality` _output_get "NewEnumerator0")
    (`MaterialInstanceDynamic.SetVectorParameterValue` _materialinstance "BodyColor" (`local.MaleColor`))
    (bind _randomname (`self.InitRandomName` "NewEnumerator0"))
    (set `self.InfoStruct` (make `/Game/Empiria/Structs/HumanPawnInfo` "NewEnumerator0" _randomname))
    (else
      (`MaterialInstanceDynamic.SetVectorParameterValue` _materialinstance "BodyColor" (`local.FemaleColor`))
      (bind _randomname_2 (`self.InitRandomName` "NewEnumerator1"))
      (set `self.InfoStruct` (make `/Game/Empiria/Structs/HumanPawnInfo` "NewEnumerator1" _randomname_2)))))

(fn `UserConstructionScript`
  (`self.RandomCharacterFeatures`))