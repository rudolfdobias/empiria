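; AbstractBuilding is a building Blueprint, apparently a base class, that shows a UI display box when clicked.
; The construction script applies DisplayMesh to the static mesh, and GetFriendlyName exposes the building's name.
; ShowDisplayBox creates a DisplayBoxClass widget bound to the building and caches it.
; As wired, it creates another when the cached box is both visible and in the viewport, and does nothing for a hidden one.
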(event `BuildingClicked`
  (`self.ShowDisplayBox`))

(fn `GetFriendlyName`
  (returns (DisplayName :type String))
  (return (`self.FriendlyName`)))

(fn `ShowDisplayBox`
  (bind _displayboxreference (`self.DisplayBoxReference`))
  (if (== _displayboxreference null)
    (bind _returnvalue (`|CreateWidget` (`self.DisplayBoxClass`) null self :!label _label))
    (bind _output_get (set `self.DisplayBoxReference` _returnvalue))
    (`UserWidget.AddToViewport` _output_get 0)
    (elif (not (or (not (`Widget.IsVisible` _displayboxreference)) (not (`Widget.IsInViewport` _displayboxreference))))
      (goto _label))))

(fn `UserConstructionScript`
  (`StaticMeshComponent.SetStaticMesh` (`self.StaticMesh`) (`self.DisplayMesh`)))