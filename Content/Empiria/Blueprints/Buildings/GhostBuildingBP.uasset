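; Ghost preview actor for placing buildings, showing the pending building's mesh at the grid-snapped cursor position.
; StartBuildingPlacement briefly spawns the building to copy its mesh and construction proxy, then activates the ghost and the controller's building mode.
; Tick gates drive movement and yaw rotation, tinting the glow by building overlap and a five-point line-trace slope check.
; GetConstructionStruct packages class, proxy, transform and mesh for construction.
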(event `self.ReceiveTick`
  (params (DeltaSeconds :type "Float (single-precision)"))
  (bind _controllerreference (`self.ControllerReference`))
  ;[1 1 1] TICK
  (`|ExecutionSequence`
    (:`then_0`
      ;[1 1 1] Building placement
      (`/Engine/EditorBlueprintResources/StandardMacros.Gate` true :!label _label
        (:`Exit`
          (set `self.CursorWorldLocation` (`/Game/Empiria/Libs/Functions.GetCursorWorldPosition` _controllerreference (`/Game/Empiria/Blueprints/Base/CameraPawnController.GetSightDistance` _controllerreference)))
          (`self.K2_SetActorLocation` self (`self.SetGridSnapVector`) false false)
          (if (or (`self.CheckIsOverlapping`) (`self.CheckSlopePlacement`))
            (set `self.CanBeBuilt` false)
            (`self.SetMeshGlow` (`self.GlowError`))
            (else
              (set `self.CanBeBuilt` true)
              (`self.SetMeshGlow` (`self.GlowOK`)))))))
    (:`then_1`
      ;[1 1 1] Building rotation
      (`/Engine/EditorBlueprintResources/StandardMacros.Gate` true :!label _label_2
        (:`Exit`
          (`self.RotateBuilding` (stale `StartBuildingRotation` ReverseDirection)))))))

(event `OpenBuildingPlacementGate`
  ;[1 1 1] Building placement
  (goto _label :!via `Open`))

(event `CloseBuildingPlacementGate`
  ;[1 1 1] Building placement
  (goto _label :!via `Close`))

(event `OnSpawn`
  (params (DisplayMesh :type "StaticMesh Object Reference") (BuildingClass :type "/Game/Empiria/Blueprints/Buildings/AbstractBuilding Class Reference") (ConstructionProxy :type "/Game/Empiria/Blueprints/Construction/ConstructionProxyBP Class Reference"))
  ;[1 1 1] Create
  (if (not (`self.IsActive`))
    (set `self.BuildingClass` BuildingClass)
    (set `self.ConstructionProxy` ConstructionProxy)
    (bind _output_get (set `self.DisplayMesh` DisplayMesh))
    (set `self.IsActive` true)
    (`StaticMeshComponent.SetStaticMesh` (`self.GhostBuilding_Mesh`) _output_get)
    (set `/Game/Empiria/Blueprints/Base/CameraPawnController.BuildingModeActive` true (`self.ControllerReference`))
    (`self.OpenBuildingPlacementGate`)
    (set `self.Extent` (`.BoxExtent` (`KismetSystemLibrary.GetComponentBounds` (`self.GhostBuilding_Mesh`))))))

(event `KillGhost`
  ;[1 1 1] Kill
  (set `self.BuildingClass` null)
  (set `self.ConstructionProxy` null)
  (`self.CloseBuildingPlacementGate`)
  (set `self.DisplayMesh` null)
  (set `self.IsActive` false)
  (set `/Game/Empiria/Blueprints/Base/CameraPawnController.BuildingModeActive` false (`self.ControllerReference`))
  (`StaticMeshComponent.SetStaticMesh` (`self.GhostBuilding_Mesh`) null))

(event `StartBuildingRotation`
  (params (ReverseDirection :type Boolean))
  ;[1 1 1] Building rotation
  (goto _label_2 :!via `Open`))

(event `EndBuildingRotation`
  ;[1 1 1] Building rotation
  (goto _label_2 :!via `Close`))

(event `/Game/Empiria/Blueprints/Interfaces/IHud.StartBuildingPlacement`
  (params (MainBuilding :type "/Game/Empiria/Blueprints/Buildings/AbstractBuilding Class Reference"))
  ;[1 1 1] StartPlacingBuilding
  (bind _returnvalue (`|SpawnActorFromClass` MainBuilding (`KismetMathLibrary.MakeTransform` (`/Game/Empiria/Libs/Functions.GetCursorWorldPosition` (`self.ControllerReference`) 2000.0)) "Undefined" "OverrideRootScale"))
  (`|ExecutionSequence`
    (:`then_0`
      (bind _asabstract_building (castclass `/Game/Empiria/Blueprints/Buildings/AbstractBuilding` MainBuilding))
      (`self.KillGhost`)
      (`self.OnSpawn` (`/Game/Empiria/Blueprints/Buildings/AbstractBuilding.DisplayMesh` _returnvalue) _asabstract_building (`/Game/Empiria/Blueprints/Buildings/AbstractBuilding.ConstructionProxy` _returnvalue)))
    (:`then_1`
      (`self.K2_DestroyActor` _returnvalue))))

(fn `CheckIsOverlapping`
  (returns (IsOverlapping :type Boolean))
  (return (> (`KismetArrayLibrary.Array_Length` (`self.GetOverlappingActors` "/Game/Empiria/Blueprints/Buildings/AbstractBuilding.AbstractBuilding_C")) 0)))

(fn `CheckSlopePlacement`
  (returns (IsInvalidLocation :type Boolean))
  (locals (Diffs :type "Array of Float (double-precision)") (MaxDiffs :type "Float (double-precision)" :default 50.0))
  (bind (_actorlocation _forwardvector _rightvector) (`self.GetVectors`))
  (bind (_actorlocation_2 _forwardvector_2 _rightvector_2) (`self.GetVectors`))
  (bind (_actorlocation_3 _forwardvector_3 _rightvector_3) (`self.GetVectors`))
  (bind (_actorlocation_4 _forwardvector_4 _rightvector_4) (`self.GetVectors`))
  (bind _actorlocation_5 (`self.GetVectors`))
  (bind _diffs (`local.Diffs`))
  (bind (_extent_x _extent_y) (`KismetMathLibrary.BreakVector` (`self.Extent`)))
  (bind _maxdiffs (`local.MaxDiffs`))
  (bind (_indexofminvalue _minvalue) (`KismetMathLibrary.MinOfFloatArray` _diffs))
  (bind (_indexofmaxvalue _maxvalue) (`KismetMathLibrary.MaxOfFloatArray` _diffs))
  (`|ExecutionSequence`
    (:`then_0`
      (`|ExecutionSequence`
        (:`then_0`
          (bind _difference (`self.SlopeTrace` (+ _actorlocation (* (+ _forwardvector _rightvector) (`self.Extent`)))))
          (`KismetArrayLibrary.Array_Add` (`local.Diffs`) _difference))
        (:`then_1`
          (bind _difference_2 (`self.SlopeTrace` (+ _actorlocation_2 (* (+ (* _forwardvector_2 -1.0) _rightvector_2) (`self.Extent`)))))
          (`KismetArrayLibrary.Array_Add` (`local.Diffs`) _difference_2))
        (:`then_2`
          (bind _difference_3 (`self.SlopeTrace` (+ _actorlocation_3 (* (+ _forwardvector_3 (* _rightvector_3 -1.0)) (`self.Extent`)))))
          (`KismetArrayLibrary.Array_Add` (`local.Diffs`) _difference_3))
        (:`then_3`
          (bind _difference_4 (`self.SlopeTrace` (+ _actorlocation_4 (* (+ (* _forwardvector_4 -1.0) (* _rightvector_4 -1.0)) (`self.Extent`)))))
          (`KismetArrayLibrary.Array_Add` (`local.Diffs`) _difference_4))
        (:`then_4`
          (bind _difference_5 (`self.SlopeTrace` (`self.GetVectors`)))
          (`KismetArrayLibrary.Array_Add` (`local.Diffs`) _difference_5))))
    (:`then_1`
      (if (and (> _indexofminvalue 0) (> _indexofmaxvalue 0))
        (bind (_outhit _returnvalue) (`KismetSystemLibrary.BoxTraceSingle` (+ _actorlocation_5 (0.0 0.0 1000.0)) (- _actorlocation_5 (0.0 0.0 1000.0)) (`KismetMathLibrary.MakeVector` _extent_x _extent_y 1.0) (struct) "TraceTypeQuery1"))))
    (:`then_2`
      (return (or (> (`KismetMathLibrary.Abs` _minvalue) _maxdiffs) (> (`KismetMathLibrary.Abs` _maxvalue) _maxdiffs))))))

(fn `GetConstructionStruct`
  (returns (ConstructionStruct :type "/Game/Empiria/Structs/ConstructionStruct Structure"))
  (return (make `/Game/Empiria/Structs/ConstructionStruct` (`self.BuildingClass`) (`self.ConstructionProxy`) (`KismetMathLibrary.MakeTransform` (`self.K2_GetActorLocation`) (`self.K2_GetActorRotation`)) (`self.DisplayMesh`))))

(fn `GetVectors`
  (returns (ActorLocation :type "Vector Structure") (ForwardVector :type "Vector Structure") (RightVector :type "Vector Structure"))
  (bind _returnvalue (`self.K2_GetActorRotation`))
  (return (`self.K2_GetActorLocation`) (`KismetMathLibrary.GetForwardVector` _returnvalue) (`KismetMathLibrary.GetRightVector` _returnvalue)))

(fn `RotateBuilding`
  (params (ReverseDirection :type Boolean))
  (locals (RotationIncrement :type "Float (double-precision)"))
  (bind _rotationsensitivity (`self.RotationSensitivity`))
  (if ReverseDirection
    (set `local.RotationIncrement` (* _rotationsensitivity -1.0))
    (else
      (set `local.RotationIncrement` _rotationsensitivity)))
  (`self.K2_SetActorRotation` (`KismetMathLibrary.MakeRotator` (.roll (`self.K2_GetActorRotation`)) (.pitch (`self.K2_GetActorRotation`)) (+ (.yaw (`self.K2_GetActorRotation`)) (`local.RotationIncrement`)))))

(fn `SetGridSnapVector`
  (returns (GridSnap :type "Vector Structure"))
  (locals (NewLocalVar_0 :type Integer))
  (bind (_cursorworldlocation_x _cursorworldlocation_y _cursorworldlocation_z) (`KismetMathLibrary.BreakVector` (`self.CursorWorldLocation`)))
  (bind _gridsize (`self.GridSize`))
  (return (`KismetMathLibrary.MakeVector` (`/Game/Empiria/Libs/Functions.GridSnap` _cursorworldlocation_x _gridsize) (`/Game/Empiria/Libs/Functions.GridSnap` _cursorworldlocation_y _gridsize) (`/Game/Empiria/Libs/Functions.GridSnap` _cursorworldlocation_z _gridsize))))

(fn `SetMeshGlow`
  (params (Color :type "Vector Structure"))
  (locals (MID :type "MaterialInstanceDynamic Object Reference"))
  (`MeshComponent.SetVectorParameterValueOnMaterials` (`self.GhostBuilding_Mesh`) "EmitColor" Color))

(fn `SlopeTrace`
  (params (TraceLocation :type "Vector Structure"))
  (returns (Difference :type "Float (double-precision)"))
  (bind (_returnvalue_x _returnvalue_y _returnvalue_z) (`KismetMathLibrary.BreakVector` (`self.K2_GetActorLocation`)))
  (bind _outhit (`KismetSystemLibrary.LineTraceSingle` (+ TraceLocation (0.0 0.0 1000.0)) (- TraceLocation (0.0 0.0 1000.0)) "TraceTypeQuery3"))
  (return (- _returnvalue_z (.z (`.ImpactPoint` (`GameplayStatics.BreakHitResult` _outhit))))))

(fn `UserConstructionScript`)