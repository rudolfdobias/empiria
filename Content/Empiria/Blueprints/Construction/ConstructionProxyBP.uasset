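; Construction site proxy that shows a glowing display mesh for a building while workers construct it.
; Constructors register and leave through report functions, and each Tick adds game-time delta multiplied by their count to the work time spent.
; Once that reaches the building class's default ConstructionTime, Tick calls ConstructionCompleted.
; GetWorkPercentage exposes progress as the ratio of time spent to required time.
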(event `self.ReceiveTick`
  (params (DeltaSeconds :type "Float (single-precision)"))
  (bind _constructioninfo_buildingclass (break `/Game/Empiria/Structs/ConstructionStruct` (`self.ConstructionInfo`)))
  (`self.DoContstructionWork` 0.0)
  (if (>= (`self.WorkTimeSpent`) (`.ConstructionTime` (defaults `/Game/Empiria/Blueprints/Construction/ConstructionProxyBP` _constructioninfo_buildingclass)))
    (`self.ConstructionCompleted` self)))

(fn `DoContstructionWork`
  (params (DeltaSecondTick :type "Float (double-precision)"))
  (locals (NumWorkers :type Integer))
  (bind _output_get (set `local.NumWorkers` (`KismetArrayLibrary.Array_Length` (`self.Constructors`))))
  (if (<= _output_get 0)
    (return)
    (else
      (bind _returnvalue (`/Game/Empiria/Blueprints/Base/EmpiriaGameState.GetDeltaGameTime` (`self.GameStateRef`) DeltaSecondTick))
      (set `self.WorkTimeSpent` (+ (* _returnvalue (`KismetMathLibrary.Conv_IntToDouble` (`local.NumWorkers`))) (`self.WorkTimeSpent`)))
      (return))))

(fn `GetWorkPercentage`
  (returns (Progress :type "Float (double-precision)"))
  (bind _constructioninfo_buildingclass (break `/Game/Empiria/Structs/ConstructionStruct` (`self.ConstructionInfo`)))
  (return (/ (`KismetMathLibrary.GetTotalMilliseconds` (`self.WorkTimeSpent`)) (`KismetMathLibrary.GetTotalMilliseconds` (`.ConstructionTime` (defaults `/Game/Empiria/Blueprints/Construction/ConstructionProxyBP` _constructioninfo_buildingclass))))))

(fn `LeaveConstruction`
  (params (Constructor :type "/Game/Empiria/Blueprints/AI/HumanBP Object Reference (by ref)"))
  (`KismetArrayLibrary.Array_RemoveItem` (`self.Constructors`) Constructor)
  (return))

(fn `ReportToConstruction`
  (params (Constructor :type "/Game/Empiria/Blueprints/AI/HumanBP Object Reference"))
  (`KismetArrayLibrary.Array_Add` (`self.Constructors`) Constructor)
  (return))

(fn `UserConstructionScript`
  (`StaticMeshComponent.SetStaticMesh` (`self.StaticMesh`) (`self.DisplayMesh`))
  (`/Game/Empiria/Libs/Functions.SetMeshGlow` (struct :`R` 0.180651 :`G` 0.183779 :`B` 0.42 :`A` 1.0) (`self.StaticMesh`)))