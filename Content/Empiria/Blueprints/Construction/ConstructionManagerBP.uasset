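; Construction manager that turns queued build requests into finished buildings through placeholder proxy actors.
; QueueConstruction spawns a proxy with the requested display mesh and transform, binds its completion event, and stores proxy and request in parallel arrays.
; When a proxy reports completion, FinishConstruction looks up its request by matching index, removes both entries, spawns the building class at that transform and destroys the proxy.
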(event `BindConstructionComplete`
  (params (Proxy :type "/Game/Empiria/Blueprints/Construction/ConstructionProxyBP Object Reference"))
  (add `/Game/Empiria/Blueprints/Construction/ConstructionProxyBP.ConstructionCompleted` Proxy (`|CreateDelegate` :!event `ConstructionCompleted`)))

(event `ConstructionCompleted`
  (params (Proxy :type "/Game/Empiria/Blueprints/Construction/ConstructionProxyBP Object Reference"))
  (`self.FinishConstruction` Proxy))

(fn `FinishConstruction`
  (params (Proxy :type "/Game/Empiria/Blueprints/Construction/ConstructionProxyBP Object Reference"))
  (locals (Idx :type Integer :default 0))
  (bind _idx (`local.Idx`))
  (bind (_buildingclass _proxyclass _transform) (break `/Game/Empiria/Structs/ConstructionStruct` (`self.Config`)))
  (bind _output_get (set `local.Idx` (`KismetArrayLibrary.Array_Find` (`self.Proxies`) Proxy)))
  (set `self.Config` (`KismetArrayLibrary.Array_Get` (`self.Queue`) _output_get))
  (`KismetArrayLibrary.Array_Remove` (`self.Queue`) _idx)
  (`KismetArrayLibrary.Array_Remove` (`self.Proxies`) _idx)
  (`|SpawnActorFromClass` _buildingclass _transform "Undefined" "OverrideRootScale")
  (`self.K2_DestroyActor` Proxy))

(fn `QueueConstruction`
  (params (ConstructionStruct :type "/Game/Empiria/Structs/ConstructionStruct Structure"))
  (bind (_buildingclass _proxyclass _transform _displaymesh) (break `/Game/Empiria/Structs/ConstructionStruct` ConstructionStruct))
  (bind _returnvalue (`|SpawnActorFromClass` _proxyclass _transform "AlwaysSpawn" "OverrideRootScale" null _displaymesh))
  (`self.BindConstructionComplete` _returnvalue)
  (`KismetArrayLibrary.Array_Add` (`self.Proxies`) _returnvalue)
  (`KismetArrayLibrary.Array_Add` (`self.Queue`) ConstructionStruct))

(fn `UserConstructionScript`)